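; Decorative actor that procedurally builds a row of randomized books from a single target mesh.
; The construction script adds Num static mesh components along local Y, spaced by mesh bounds, Distance and each book's random scale.
; Each gets random rotation, with height either aligned from scaled bounds via AlignZ or randomly offset.
; A dynamic material instance per book receives a random Index parameter to vary its appearance.
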(event EventBeginPlay)

(event Collision|EventActorBeginOverlap
  (params (OtherActor :type Actor%20Object%20Reference)))

(event EventTick
  (params (DeltaSeconds :type Float%20%28single-precision%29)))

(fn ConstructionScript
  (bind _scale_random (Variables|Default|GetScale%20Random))
  (bind _offset_random (Variables|Default|GetOffset%20Random))
  (bind _randomrotation_yaw (Variables|Default|GetRandomRotation_Yaw))
  (bind _randomrotation_pitch (Variables|Default|GetRandomRotation_Pitch))
  (bind _randomrotation_roll (Variables|Default|GetRandomRotation_Roll))
  (Utilities|FlowControl|Sequence
    (:then_1
      (for _index (range 0 (- (Variables|Default|GetNum) 1))
        (LocalVariables|SetScale (Math|Random|RandomFloatinRange (.x _scale_random) (.y _scale_random)))
        (LocalVariables|SetRandom%20Yaw (Math|Random|RandomFloatinRange (.x _randomrotation_yaw) (.y _randomrotation_yaw)))
        (LocalVariables|SetRandom%20Pitch (Math|Random|RandomFloatinRange (.x _randomrotation_pitch) (.y _randomrotation_pitch)))
        (LocalVariables|SetRandom%20Roll (Math|Random|RandomFloatinRange (.x _randomrotation_roll) (.y _randomrotation_roll)))
        (bind _returnvalue (AddComponent|AddStaticMeshComponent false (Math|Transform|MakeTransform (Math|Vector|MakeVector 0.0 (* _index (+ (.Y (Math|Vector|BreakVector (.boxextent (StaticMesh|GetBounds (Variables|Default|GetTarget%20Book%20Mesh))))) (Variables|Default|GetDistance)) 2.0 (LocalVariables|GetScale)) (Math|Float|SelectFloat (* (LocalVariables|GetScale) (.Z (Math|Vector|BreakVector (.BoxExtent (Math|BoxSphereBounds|BreakBoxSphereBounds (StaticMesh|GetBounds (Variables|Default|GetTarget%20Book%20Mesh))))))) (Math|Random|RandomFloatinRange (.x _offset_random) (.y _offset_random)) (Variables|Default|GetAlign%20Z))) (Math|Rotator|MakeRotator (LocalVariables|GetRandom%20Roll) (LocalVariables|GetRandom%20Pitch) (LocalVariables|GetRandom%20Yaw)) (Math|Conversions|ToVector(Float) (LocalVariables|GetScale)))))
        (Components|StaticMesh|SetStaticMesh _returnvalue (Variables|Default|GetTarget%20Book%20Mesh))
        (bind _returnvalue_2 (Rendering|Material|CreateDynamicMaterialInstance (Variables|Default|GetTarget%20MasterMaterial) "None" "None" :!class /Script/Engine.KismetMaterialLibrary))
        (Rendering|Material|SetMaterial _returnvalue 0 _returnvalue_2)
        (Rendering|Material|SetScalarParameterValue _returnvalue_2 "Index" (Math|Conversions|ToFloat(Integer) (Math|Random|RandomIntegerinRange 0 23)) :!class /Script/Engine.MaterialInstanceDynamic)))))