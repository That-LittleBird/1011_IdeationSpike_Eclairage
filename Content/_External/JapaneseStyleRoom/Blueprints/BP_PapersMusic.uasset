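; BP_PapersMusic is a decorative prop from a Japanese-style room pack that randomizes its look, apparently a sheet-music paper.
; The construction script picks a random mesh from an array and applies a random yaw within a configurable range.
; It assigns a dynamic material instance and sets a random Index parameter to vary the material per placed actor.
; The event graph holds only disabled stub events, so nothing runs at play time.
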(event EventBeginPlay)

(event Collision|EventActorBeginOverlap
  (params (OtherActor :type Actor%20Object%20Reference)))

(event EventTick
  (params (DeltaSeconds :type Float%20%28single-precision%29)))

(fn ConstructionScript
  (bind _staticmesh (Variables|Default|GetStaticMesh))
  (bind _random_rotation (Variables|Default|GetRandom%20Rotation))
  (Components|StaticMesh|SetStaticMesh _staticmesh (.OutItem (Utilities|Array|Random (Variables|Default|GetMeshs))))
  (bind _returnvalue (Rendering|Material|CreateDynamicMaterialInstance (Variables|Default|GetTargetMaterials) "None" "None" :!class /Script/Engine.KismetMaterialLibrary))
  (Rendering|Material|SetMaterial _staticmesh 0 _returnvalue)
  (Transformation|SetRelativeRotation _staticmesh (Math|Rotator|MakeRotator 0.0 0.0 (Math|Random|RandomFloatinRange (.x _random_rotation) (.y _random_rotation))) false false)
  (Rendering|Material|SetScalarParameterValue _returnvalue "Index" (Math|Conversions|ToFloat(Integer) (Math|Random|RandomIntegerinRange 0 19)) :!class /Script/Engine.MaterialInstanceDynamic))