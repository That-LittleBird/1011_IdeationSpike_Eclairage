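; BP_SwitchLine is a spline-driven line prop for the Japanese-style room, likely a wire running to a switch.
; Its construction script adds spline mesh components between consecutive spline points, using their local positions and tangents.
; When UseLineCach is on, it also places static meshes, apparently line clips, every LineCachDis along the spline using world-space transforms and manual attachment.
; The event graph has no active logic.
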(event EventBeginPlay)

(event Collision|EventActorBeginOverlap
  (params (OtherActor :type Actor%20Object%20Reference)))

(event EventTick
  (params (DeltaSeconds :type Float%20%28single-precision%29)))

(fn ConstructionScript
  (bind _spline (Variables|Default|GetSpline))
  (bind _spline_2 (Variables|Default|GetSpline))
  (bind _spline_3 (Variables|Default|GetSpline))
  (for _index (range 1 (Spline|GetNumberOfSplinePoints _spline))
    (bind _returnvalue (AddComponent|AddSplineMeshComponent false))
    (SplineMesh|SetStartandEnd _returnvalue (.Location (Spline|GetLocationandTangentatSplinePoint _spline_3 (- _index 1) "Local")) (.Tangent (Spline|GetLocationandTangentatSplinePoint _spline_3 (- _index 1) "Local")) (.Location (Spline|GetLocationandTangentatSplinePoint _spline_3 _index "Local")) (.Tangent (Spline|GetLocationandTangentatSplinePoint _spline_3 _index "Local")) true :!class /Script/Engine.SplineMeshComponent))
  (if (Variables|Default|GetUse%20LineCach)
    (for _index_2 (range 1 (Math|Float|Ceil (/ (Spline|GetSplineLength _spline) (Variables|Default|GetLineCachDis))))
      (AddComponent|AddStaticMeshComponent true (Math|Transform|MakeTransform (Spline|GetLocationatDistanceAlongSpline _spline_2 (* _index_2 (Variables|Default|GetLineCachDis)) "World") (Spline|GetRotationatDistanceAlongSpline _spline_2 (* _index_2 (Variables|Default|GetLineCachDis)) "World"))))))